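; GA_FireBolt is a gameplay ability that casts a fire bolt projectile toward the point under the mouse.
; On valid target data, it sends the avatar a facing update and picks a random tagged attack montage, ending if none is returned.
; It waits for the montage's tagged gameplay event, then spawns the projectile with that montage's socket tag and target location and ends.
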(event Ability|EventOnEndAbility
  (params (bWasCancelled :type Boolean)))

(event Ability|EventActivateAbility
  (bind _datahandle (|TargetDataUnderMouse)
    (:ValidData
      (Variables|Default|SetProjectileTargetLocation (.Location (Collision|BreakHitResult (Ability|TargetData|GetHitResultfromTargetData _datahandle))))
      (Class|CombatInterface|UpdateFacingTarget(Message) (Ability|GetAvatarActorfromActorInfo) (Variables|Default|GetProjectileTargetLocation))
      (bind _returnvalue (Class|CombatInterface|GetAttackMontages(Message) (Ability|GetAvatarActorfromActorInfo)))
      (Variables|Default|SetTaggedMontage (.OutTaggedMontage (Class|DamageGameplayAbility|GetRandomTaggedMontagefromArray _returnvalue)))
      (if (.ReturnValue (Class|DamageGameplayAbility|GetRandomTaggedMontagefromArray _returnvalue))
        (|PlayMontageandWaitProxy "None" (.Montage (Utilities|Struct|BreakTaggedMontage (Variables|Default|GetTaggedMontage))) 1.0 "None" true 1.0 0.0 false
          (:then
            (Ability|Tasks|WaitGameplayEvent (.MontageTag (Utilities|Struct|BreakTaggedMontage (Variables|Default|GetTaggedMontage))) 0
              (:EventReceived
                (Class|DGProjectileSpell|SpawnProjectile (Variables|Default|GetProjectileTargetLocation) (.SocketTag (Utilities|Struct|BreakTaggedMontage (Variables|Default|GetTaggedMontage))) false 0.0)
                (Ability|EndAbility)))))
        (else
          (Ability|EndAbility))))))