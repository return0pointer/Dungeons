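; Hero gameplay ability that performs a dodge jump with temporary invulnerability and a trailing shadow effect.
; If CanJump, it plays the avatar's jump montage and waits for In and Out gameplay-event tags.
; In toggles invulnerability on with a visibility change, attaches a Niagara effect and starts a looping timer that spawns shadow actors at the character's mesh.
; Out reverses these, then ends the ability after a short delay.
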(event Custom|StartShadowSpawnTimer
  ;[0 0.1034 1] Shadow Spawn
  (bind _returnvalue (Utilities|Time|SetTimerbyEvent (delegate Custom|SpawnTrail) 0.05 true))
  (Variables|Default|SetShadowTimerHandle _returnvalue))

(event Custom|SpawnTrail
  ;[0 0.1034 1] Shadow Spawn
  ;;[0 0.1034 1] Spawn shadow meshes
  (Game|SpawnActorfromClass (Variables|Default|GetShadowActorClass) (Transformation|GetWorldTransform (Variables|/Script/Engine.Character|GetMesh (Variables|Default|GetCharacterToJump))) "Undefined" "MultiplyWithRoot" 0 0))

(event Ability|EventActivateAbility
  (|CallParentFunction)
  (if (Variables|Default|GetCanJump)
    (bind _returnvalue (Class|CombatInterface|GetJumpMontage(Message) (Ability|GetAvatarActorfromActorInfo)))
    (|PlayMontageandWaitProxy "None" _returnvalue 1.0 "None" false 1.0 0.0 false
      (:then
        (Ability|Tasks|WaitGameplayEvent "(TagName=\"Montage.Ability.DodgeJump.In\")" 0
          (:then
            (Ability|Tasks|WaitGameplayEvent "(TagName=\"Montage.Ability.DodgeJump.Out\")" 0
              (:EventReceived
                (Class|CombatInterface|SetInvulnerability(Message) (Ability|GetAvatarActorfromActorInfo) false true)
                ;[0 0.1034 1] Clear Shadow Timer
                (Utilities|Time|ClearandInvalidateTimerbyHandle (Variables|Default|GetShadowTimerHandle))
                (Components|DestroyComponent (Variables|Default|GetFadeEffect))
                (Utilities|FlowControl|Delay 0.5)
                (Ability|EndAbility))))
          (:EventReceived
            (bind _returnvalue_2 (Niagara|SpawnSystemAttached (Variables|Default|GetJumpEffect) (Variables|/Script/Engine.Actor|GetRootComponent (Ability|GetAvatarActorfromActorInfo)) "None" "0, 0, 0" "0, 0, 0" "KeepRelativeOffset" false))
            (Variables|Default|SetFadeEffect _returnvalue_2)
            (Class|CombatInterface|SetInvulnerability(Message) (Ability|GetAvatarActorfromActorInfo) true true)
            (CallFunction|StartShadowSpawnTimer)))))
    (else
      (Ability|EndAbility))))