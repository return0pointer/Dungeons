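; Enemy gameplay ability that summons random minions, each with a default controller, at a set of spawn locations.
; On activation it shuffles the locations, plays a ground summon Niagara effect at each and starts the cast montage.
; The montage's attack gameplay event starts a delayed loop that spawns minions one by one, facing away from the caster.
; The ability ends shortly after the last spawn.
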(event Ability|EventActivateAbility
  (Variables|Default|SetSpawnLocationIndex 0)
  (bind _returnvalue (Class|SummonAbility|GetSpawnLocation))
  (bind _output_get (Variables|Default|SetSpawnLocations _returnvalue))
  (Utilities|Array|Shuffle _output_get)
  (for _array_element _output_get
    (Niagara|SpawnSystematLocation "/Game/Assets/Effects/Combat/NS_GroundSummon.NS_GroundSummon" _array_element))
  (|PlayMontageandWaitProxy "None" "/Game/Assets/Characters/Mixamo/Character/Animations/AM_Character_CastSpawn.AM_Character_CastSpawn" 1.0 "None" true 1.0 0.0 false
    (:then
      (Ability|Tasks|WaitGameplayEvent "(TagName=\"Montage.Attack.1\")" 0
        (:EventReceived
          (if (< (Variables|Default|GetSpawnLocationIndex) (Utilities|Array|Length (Variables|Default|GetSpawnLocations))) :!label _label
            (bind _returnvalue_2 (Game|SpawnActorfromClass (Class|SummonAbility|GetRandomMinionClass) (Math|Transform|MakeTransform (Utilities|Array|Get(acopy) (Variables|Default|GetSpawnLocations) (Variables|Default|GetSpawnLocationIndex)) (Math|Rotator|FindLookatRotation (Transformation|GetActorLocation (Ability|GetAvatarActorfromActorInfo)) (Utilities|Array|Get(acopy) (Variables|Default|GetSpawnLocations) (Variables|Default|GetSpawnLocationIndex))) "1.000000,1.000000,1.000000") "Undefined" "MultiplyWithRoot" 0 0))
            (Pawn|SpawnDefaultController _returnvalue_2)
            (Math|Integer|IncrementInt (Variables|Default|GetSpawnLocationIndex)
              (:%20%20
                (Utilities|FlowControl|Delay 0.2)
                (goto _label)))
            (else
              (Utilities|FlowControl|Delay 1.0)
              (Ability|EndAbility))))))))