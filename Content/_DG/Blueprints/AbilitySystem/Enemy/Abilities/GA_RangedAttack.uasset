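; GA_RangedAttack is an enemy gameplay ability that fires a projectile at the avatar's combat target.
; On activation it gets the target from the avatar, faces it, and plays a random tagged attack montage.
; A gameplay event matching the montage's tag triggers the projectile spawn from that montage's socket toward the target's current location, then the ability ends after a short delay.
; It also ends if no montage is found or playback completes, is interrupted or cancelled.
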(event Ability|EventActivateAbility
  (bind _returnvalue (Ability|GetAvatarActorfromActorInfo))
  (bind _returnvalue_2 (Class|EnemyInterface|GetCombatTarget(Message) (Ability|GetAvatarActorfromActorInfo)))
  (Variables|Default|SetTargetActor _returnvalue_2)
  (Class|CombatInterface|UpdateFacingTarget(Message) _returnvalue (Transformation|GetActorLocation _returnvalue_2))
  (bind _returnvalue_3 (Class|CombatInterface|GetAttackMontages(Message) _returnvalue))
  (if (.ReturnValue (Class|DamageGameplayAbility|GetRandomTaggedMontagefromArray _returnvalue_3))
    (Variables|Default|SetTaggedMontage (.OutTaggedMontage (Class|DamageGameplayAbility|GetRandomTaggedMontagefromArray _returnvalue_3)))
    (|PlayMontageandWaitProxy "None" (.Montage (Utilities|Struct|BreakTaggedMontage (Variables|Default|GetTaggedMontage))) 1.0 "None" false 1.0 0.0 false
      (:then
        (Ability|Tasks|WaitGameplayEvent (.MontageTag (Utilities|Struct|BreakTaggedMontage (Variables|Default|GetTaggedMontage))) 0
          (:EventReceived
            (Class|DGProjectileSpell|SpawnProjectile (Transformation|GetActorLocation (Variables|Default|GetTargetActor)) (.SocketTag (Utilities|Struct|BreakTaggedMontage (Variables|Default|GetTaggedMontage))))
            (Utilities|FlowControl|Delay 0.2)
            (Ability|EndAbility))))
      (:OnCompleted
        (Ability|EndAbility :!label _label))
      (:OnInterrupted
        (goto _label))
      (:OnCancelled
        (goto _label)))
    (else
      (goto _label))))