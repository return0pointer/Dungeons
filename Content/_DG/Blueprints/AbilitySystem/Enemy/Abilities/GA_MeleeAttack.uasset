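; Enemy melee attack gameplay ability that plays a random tagged attack montage while facing the combat target.
; When the montage's gameplay event arrives, it searches a small sphere at the matching combat socket for live players.
; Non-friendly hits take damage and spawn their blood effect, with one impact sound if anything was hit.
; The ability ends after the hit check or montage end, without stopping the montage.
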(event Ability|EventActivateAbility
  (bind _returnvalue (Ability|GetAvatarActorfromActorInfo))
  (bind _returnvalue_2 (Ability|GetAvatarActorfromActorInfo))
  (Variables|Default|SetHasHitTarget false)
  (bind _returnvalue_3 (Class|EnemyInterface|GetCombatTarget(Message) _returnvalue))
  (bind _ascombat_interface (Utilities|Casting|CastToCombatInterface _returnvalue))
  (Class|CombatInterface|UpdateFacingTarget _ascombat_interface (Transformation|GetActorLocation _returnvalue_3))
  (bind _returnvalue_4 (Class|CombatInterface|GetAttackMontages(Message) _returnvalue))
  (if (.ReturnValue (Class|DamageGameplayAbility|GetRandomTaggedMontagefromArray _returnvalue_4))
    (Variables|Default|SetTaggedMontage (.OutTaggedMontage (Class|DamageGameplayAbility|GetRandomTaggedMontagefromArray _returnvalue_4)))
    (|PlayMontageandWaitProxy "None" (.Montage (Utilities|Struct|BreakTaggedMontage (Variables|Default|GetTaggedMontage))) 1.0 "None" false 1.0 0.0 false
      (:then
        (Ability|Tasks|WaitGameplayEvent (.MontageTag (Utilities|Struct|BreakTaggedMontage (Variables|Default|GetTaggedMontage))) 0
          (:EventReceived
            (bind _returnvalue_5 (Class|CombatInterface|GetCombatSocketLocation(Message) _returnvalue_2 (.MontageTag (Utilities|Struct|BreakTaggedMontage (Variables|Default|GetTaggedMontage)))))
            (bind _output_get (Variables|Default|SetCombatSocketLocation _returnvalue_5))
            (bind _outoverlappingactors (Class|DGAbilitySystemLibrary|GetLivePlayersWithinRadius _returnvalue_2 6e+01 _output_get (Utilities|Array|MakeArray _returnvalue_2)))
            (for _array_element _outoverlappingactors
              (if (Class|DGAbilitySystemLibrary|IsNotFriend (Ability|GetAvatarActorfromActorInfo) _array_element)
                (Class|DamageGameplayAbility|CauseDamage _array_element)
                (Variables|Default|SetHasHitTarget true)
                (bind _returnvalue_6 (Class|CombatInterface|GetBloodEffect(Message) _array_element))
                (Niagara|SpawnSystematLocation _returnvalue_6 (Variables|Default|GetCombatSocketLocation))))
            (if (Variables|Default|GetHasHitTarget)
              (Audio|PlaySoundatLocation (.ImpactSound (Utilities|Struct|BreakTaggedMontage (Variables|Default|GetTaggedMontage))) (Variables|Default|GetCombatSocketLocation) "0, 0, 0" 1.0 1.0 0.0 0 0 0 0)))))
      (:OnCompleted
        _)
      (:OnInterrupted
        _)
      (:OnCancelled
        _)))
  (Ability|EndAbility))

(fn TryEndAbility
  (if (and (Variables|Default|GetEndDamage) (Variables|Default|GetEndMontage))
    (Ability|EndAbility)
    (Variables|Default|SetEndMontage false)
    (Variables|Default|SetEndDamage false)))