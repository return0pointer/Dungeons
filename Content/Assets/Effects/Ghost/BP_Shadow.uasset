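; BP_Shadow is a ghost afterimage effect that freezes a snapshot of the player character's pose and destroys itself when done.
; On BeginPlay a PoseableMesh takes the player's skeletal mesh, copies its current pose and applies a shadow material seeded with a random scalar.
; A timeline then drives the material's Alpha parameter, and the actor is destroyed when it finishes.
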(event EventBeginPlay
  (bind _returnvalue (Game|GetPlayerCharacter 0))
  (bind _poseablemesh (Variables|Default|GetPoseableMesh))
  (bind _mesh (Variables|/Script/Engine.Character|GetMesh _returnvalue))
  (Components|SkinnedMesh|SetSkinnedAssetandUpdate _poseablemesh (Variables|/Script/Engine.SkeletalMeshComponent|GetSkeletalMeshAsset _mesh) true)
  (Rendering|Material|SetMaterial _poseablemesh 0 "/Game/Assets/Effects/Ghost/M_Shadow_Inst.M_Shadow_Inst")
  (Rendering|Material|SetScalarParameterValueonMaterials (Variables|Default|GetPoseableMesh) "Random" (Math|Random|RandomFloat))
  (Class|PoseableMeshComponent|CopyPosefromSkeletalComponent (Variables|Default|GetPoseableMesh) _mesh)
  (bind _newtrack_0 (Timeline|Timeline PlayFromStart)
    (:Update
      (Rendering|Material|SetScalarParameterValueonMaterials (Variables|Default|GetPoseableMesh) "Alpha" _newtrack_0))
    (:Finished
      (Actor|DestroyActor))))

(event Collision|EventActorBeginOverlap
  (params (OtherActor :type Actor%20Object%20Reference)))

(event EventTick
  (params (DeltaSeconds :type Float%20%28single-precision%29)))

(fn ConstructionScript)